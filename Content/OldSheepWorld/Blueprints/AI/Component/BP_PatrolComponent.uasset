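; BP_PatrolComponent is an AI component that holds patrol data and supplies move destinations for its owning actor.
; On BeginPlay it caches the locations of valid PatrolPoints actors into PatrolLocations and sets MaxNum from the loop index.
; GetNextLocation does not read that cached list; it returns a random navigable location within a fixed radius of the owner, plus a success flag.
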(event `self.ReceiveBeginPlay`
  (bind _patrolpoints (`self.PatrolPoints`))
  (`KismetArrayLibrary.Array_Clear` (`self.PatrolLocations`))
  (if (> (`KismetArrayLibrary.Array_Length` _patrolpoints) 0)
    (for (_array_element _array_index) _patrolpoints
      (`/Engine/EditorBlueprintResources/StandardMacros.IsValid` _array_element
        (:`Is Valid`
          (`KismetArrayLibrary.Array_Add` (`self.PatrolLocations`) (`Actor.K2_GetActorLocation` _array_element)))))
    (set `self.MaxNum` _array_index)))

(fn `Get Next Location`
  (returns (Output_Get :type "Vector Structure") (FindSucess :type Boolean))
  (bind (_randomlocation _returnvalue) (`NavigationSystemV1.K2_GetRandomLocationInNavigableRadius` (`Actor.K2_GetActorLocation` (`self.GetOwner`)) 2000.0 null null))
  (return _randomlocation _returnvalue))