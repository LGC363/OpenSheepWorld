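; AI controller for the Countess enemy that runs BT_Countess and feeds the player and the pawn's health into its blackboard.
; Perception updates go to sight and damage handlers that switch the pawn's enemy state message.
; Sight of a Player-tagged actor starts or drops the chase state.
; Damage raises a separate state from the lost-sight one, targets the sensed actor and refreshes blackboard health.
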(event `self.ReceiveBeginPlay`
  (bind _blackboard (`self.Blackboard`))
  (`self.RunBehaviorTree` "/Game/OldSheepWorld/Blueprints/AI/Countess/BT_Countess.BT_Countess")
  (bind _ascountess_player_character (cast `/Game/OldSheepWorld/Blueprints/AI/Countess/CountessPlayerCharacter` (`self.K2_GetPawn`)))
  (bind _newparam (`/Game/OldSheepWorld/Blueprints/AI/Countess/CountessPlayerCharacter.GetHealth` _ascountess_player_character))
  (`BlackboardComponent.SetValueAsFloat` _blackboard "Health" _newparam)
  (`BlackboardComponent.SetValueAsObject` _blackboard "Player" (`GameplayStatics.GetPlayerCharacter` 0)))

(event `self.AIPerception Component.OnTargetPerceptionUpdated`
  (params (Actor :type "Actor Object Reference") (Stimulus :type "AIStimulus Structure"))
  (`self.OnSightSence` Actor Stimulus)
  (`self.OnDamage` Actor Stimulus))

(fn `OnDamage`
  (params (Actor :type "Actor Object Reference") (Stimulus :type "AIStimulus Structure"))
  (bind _returnvalue (`self.K2_GetPawn`))
  (bind _blackboard (`self.Blackboard`))
  (bind _returnvalue_2 (`AIPerceptionSystem.GetSenseClassForStimulus` Stimulus))
  (if (== _returnvalue_2 "/Script/AIModule.AISense_Damage")
    (if (`.bSuccessfullySensed` (break `AIStimulus` Stimulus))
      (bind _currentenemystate (message `/Game/OldSheepWorld/Blueprints/AI/Interface/EnemyStateInterface.GetEnemyState` _returnvalue))
      (if (`|EnumEquality` _currentenemystate "NewEnumerator0")
        (message `/Game/OldSheepWorld/Blueprints/AI/Interface/EnemyStateInterface.SetEnemyState` _returnvalue "NewEnumerator2"))
      (`BlackboardComponent.SetValueAsObject` _blackboard "Player" (`local.Actor`))
      (bind _ascountess_player_character (cast `/Game/OldSheepWorld/Blueprints/AI/Countess/CountessPlayerCharacter` (`self.K2_GetPawn`)))
      (bind _newparam (`/Game/OldSheepWorld/Blueprints/AI/Countess/CountessPlayerCharacter.GetHealth` _ascountess_player_character))
      (`BlackboardComponent.SetValueAsFloat` _blackboard "Health" _newparam)
      (bind _ascountess_player_character_2 (cast `/Game/OldSheepWorld/Blueprints/AI/Countess/CountessPlayerCharacter` (`self.K2_GetPawn`)))
      (set `self.Damage` (`/Game/OldSheepWorld/Blueprints/AI/Countess/CountessPlayerCharacter.Damage` _ascountess_player_character_2)))))

(fn `OnSightSence`
  (params (Actor :type "Actor Object Reference") (Stimulus :type "AIStimulus Structure"))
  (bind _returnvalue (`self.K2_GetPawn`))
  (bind _returnvalue_2 (`AIPerceptionSystem.GetSenseClassForStimulus` Stimulus))
  (if (== _returnvalue_2 "/Script/AIModule.AISense_Sight")
    (if (`self.ActorHasTag` Actor "Player")
      (if (`.bSuccessfullySensed` (break `AIStimulus` (`local.Stimulus`)))
        (message `/Game/OldSheepWorld/Blueprints/AI/Interface/EnemyStateInterface.SetEnemyState` _returnvalue "NewEnumerator1")
        (`KismetSystemLibrary.PrintString` "Begin Chase")
        (`BlackboardComponent.SetValueAsObject` (`self.Blackboard`) "Player" (`local.Actor`))
        (else
          (message `/Game/OldSheepWorld/Blueprints/AI/Interface/EnemyStateInterface.SetEnemyState` _returnvalue "NewEnumerator0")
          (`KismetSystemLibrary.PrintString` "Lose Sight"))))))

(fn `UserConstructionScript`)