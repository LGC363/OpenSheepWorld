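; Player character with switchable rifle, pistol and unarmed stances, each linking its own animation class layers.
; Primary attack in armed stances fires projectiles on montage notifies, aimed by camera trace from the spawn point, with cooldown until montage completion.
; Right mouse eases the camera between two spring arms for aiming.
; Damage drains clamped health; at zero it disables collision and input, plays a death montage, calls a dispatcher, then destroys the actor.
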(event `EnhancedInput|/Game/OldSheepWorld/Input/Actions/IA_MontageTest01`
  (params (ActionValue :type "Vector2D Structure") (ElapsedSeconds :type "Float (double-precision)") (TriggeredSeconds :type "Float (double-precision)") (InputAction :type "InputAction Object Reference" :default "/Game/OldSheepWorld/Input/Actions/IA_MontageTest01.IA_MontageTest01"))
  ;[1 1 1] MontageTest01
  (:`Started`
    (`KismetSystemLibrary.PrintString` "PlayMontageBegin")
    (`|PlayMontage` (`self.Mesh`) "/Game/EgyptGirl/Animations/Actions/AM_Test01.AM_Test01" 1.0 0.0 "start"
      (:`OnNotifyBegin`
        (`|PlayMontage` (`self.Mesh`) "/Game/EgyptGirl/Animations/Actions/AM_Test02.AM_Test02" 1.0 0.0 "start"
          (:`OnCompleted`
            (`KismetSystemLibrary.PrintString` "PlayMontageEnd")))))))

(event `self.ReceiveAnyDamage`
  (params (Damage :type "Float (single-precision)") (DamageType :type "DamageType Object Reference") (InstigatedBy :type "Controller Object Reference") (DamageCauser :type "Actor Object Reference"))
  (bind _returnvalue (`GameplayStatics.GetPlayerController` 0))
  (bind _output_get (set `self.Health` (`KismetMathLibrary.FClamp` (- (`self.Health`) Damage) 0.0 (`self.MaxHealth`))))
  (if (<= _output_get 0.0)
    (`PrimitiveComponent.SetCollisionEnabled` (`self.Mesh`) "NoCollision")
    (`PrimitiveComponent.SetCollisionEnabled` (`self.CapsuleComponent`) "NoCollision")
    (`|PlayMontage` (`self.Mesh`) "/Game/OldSheepWorld/Blueprints/Montage/PlayerCharacter/AM_Death.AM_Death" 1.0 0.0 "death"
      (:`then`
        (`self.DisableInput` _returnvalue))
      (:`OnCompleted`
        (`self.EnableInput` _returnvalue)
        (`self.DeathDispatcher`)
        (`self.K2_DestroyActor`)))))

(event `self.ReceiveBeginPlay`
  ;[1 1 1] BeginPlay
  (`SkeletalMeshComponent.LinkAnimClassLayers` (`self.Mesh`) "/Game/EgyptGirl/Animations/ABP_RifleLayers.ABP_RifleLayers_C") ; 关联动画类图层，让其和另一个动画图层进行关联
  (set `self.InState2` false)
  (set `self.InState1` true)
  (set `self.InState3` false))

(event `Key|RightMouseButton`
  (params (Key :type "Key Structure"))
  (bind _followcamera (`self.FollowCamera`))
  (bind _followcamera_2 (`self.FollowCamera`))
  (:`Pressed`
    (`SceneComponent.K2_AttachToComponent` _followcamera_2 (`self.SpringArm`) "None" "KeepWorld" "KeepWorld" "KeepWorld" true)
    (`KismetSystemLibrary.MoveComponentTo` _followcamera_2 (0.0 0.0 0.0) (struct :`Pitch` -20.0) true true 0.1))
  (:`Released`
    (`SceneComponent.K2_AttachToComponent` _followcamera (`self.CameraBoom`) "None" "KeepWorld" "KeepWorld" "KeepWorld" true)
    (`KismetSystemLibrary.MoveComponentTo` _followcamera (20.0 100.0 160.0) (struct :`Pitch` -20.0) true true 0.1)))

(event `EnhancedInput|/Game/OldSheepWorld/Input/Actions/IA_SwitchToState01`
  (params (ActionValue :type Boolean) (ElapsedSeconds :type "Float (double-precision)") (TriggeredSeconds :type "Float (double-precision)") (InputAction :type "InputAction Object Reference" :default "/Game/OldSheepWorld/Input/Actions/IA_SwitchToState01.IA_SwitchToState01"))
  ;[1 1 1] SwitchToState01
  (:`Started`
    (if (`self.InState1`)
      (`KismetSystemLibrary.PrintString` "AlreadyInAnimLayerRifle")
      (else
        (`KismetSystemLibrary.PrintString` "SwitchToAnimLayerRifle")
        (`SkeletalMeshComponent.LinkAnimClassLayers` (`self.Mesh`) "/Game/EgyptGirl/Animations/ABP_RifleLayers.ABP_RifleLayers_C") ; 关联动画类图层，让其和另一个动画图层进行关联
        (set `self.InState2` false)
        (set `self.InState1` true)
        (set `self.InState3` false)))))

(event `EnhancedInput|/Game/OldSheepWorld/Input/Actions/IA_SwitchToState02`
  (params (ActionValue :type Boolean) (ElapsedSeconds :type "Float (double-precision)") (TriggeredSeconds :type "Float (double-precision)") (InputAction :type "InputAction Object Reference" :default "/Game/OldSheepWorld/Input/Actions/IA_SwitchToState02.IA_SwitchToState02"))
  ;[1 1 1] SwitchToState02
  (:`Started`
    (if (`self.InState2`)
      (`KismetSystemLibrary.PrintString` "AlreadyInAnimLayerPistol")
      (else
        (`KismetSystemLibrary.PrintString` "SwitchToAnimLayerPistol")
        (`SkeletalMeshComponent.LinkAnimClassLayers` (`self.Mesh`) "/Game/EgyptGirl/Animations/ABP_PistolLayers.ABP_PistolLayers_C") ; 关联动画类图层，让其和另一个动画图层进行关联
        (set `self.InState2` true)
        (set `self.InState1` false)
        (set `self.InState3` false)))))

(event `EnhancedInput|/Game/OldSheepWorld/Input/Actions/IA_SwitchToState03`
  (params (ActionValue :type Boolean) (ElapsedSeconds :type "Float (double-precision)") (TriggeredSeconds :type "Float (double-precision)") (InputAction :type "InputAction Object Reference" :default "/Game/OldSheepWorld/Input/Actions/IA_SwitchToState03.IA_SwitchToState03"))
  ;[1 1 1] SwitchToState03
  (:`Started`
    (if (`self.InState3`)
      (`KismetSystemLibrary.PrintString` "AlreadyInAnimLayerUnarm")
      (else
        (`KismetSystemLibrary.PrintString` "SwitchToAnimLayerUnarm")
        (`SkeletalMeshComponent.LinkAnimClassLayers` (`self.Mesh`) "/Game/EgyptGirl/Animations/ABP_UnarmLayers.ABP_UnarmLayers_C" :!pinned true) ; 关联动画类图层，让其和另一个动画图层进行关联
        (set `self.InState2` false)
        (set `self.InState1` false)
        (set `self.InState3` true)))))

(event `EnhancedInput|/Game/OldSheepWorld/Input/Actions/IA_PrimaryAttack`
  (params (ActionValue :type Boolean) (ElapsedSeconds :type "Float (double-precision)") (TriggeredSeconds :type "Float (double-precision)") (InputAction :type "InputAction Object Reference" :default "/Game/OldSheepWorld/Input/Actions/IA_PrimaryAttack.IA_PrimaryAttack"))
  ;[1 1 1] PrimaryAttack
  (:`Triggered`
    (if (not (`self.IsPrimaryAttackCooldown`))
      (set `self.IsPrimaryAttackCooldown` true)
      (if (`self.InState1`)
        (`|PlayMontage` (`self.Mesh`) "/Game/OldSheepWorld/Blueprints/Montage/PlayerCharacter/AM_Rifle_Fire_Montage.AM_Rifle_Fire_Montage" 2.0 0.0 "start"
          (:`OnCompleted`
            (set `self.IsPrimaryAttackCooldown` false))
          (:`OnNotifyBegin`
            (bind _returnvalue (`|SpawnActorFromClass` "/Game/OldSheepWorld/Blueprints/BP_PrimaryProj.BP_PrimaryProj_C" (`KismetMathLibrary.Conv_VectorToTransform` (`SceneComponent.K2_GetComponentLocation` (`self.ProjSpawnPosition`))) "Undefined" "OverrideRootScale" null null))
            (set `self.ProjStartLocation` (`SceneComponent.K2_GetComponentLocation` (`self.FollowCamera`)))
            (bind _output_get (set `self.ProjEndLocation` (`KismetMathLibrary.Conv_RotatorToVector` (`SceneComponent.K2_GetComponentRotation` (`self.FollowCamera`)))))
            (bind _output_get_2 (set `self.LineTraceDistance` 10000))
            (bind _output_get_3 (set `self.ProjEndLocation` (+ (* _output_get_2 (`KismetMathLibrary.Normal` _output_get)) (`self.ProjStartLocation`))))
            (bind (_outhit _returnvalue_2) (`KismetSystemLibrary.LineTraceSingle` (`self.ProjStartLocation`) _output_get_3 "TraceTypeQuery2"))
            (set `self.ProjStartLocation` (`SceneComponent.K2_GetComponentLocation` (`self.ProjSpawnPosition`)))
            (if _returnvalue_2
              (bind _output_get_4 (set `self.ProjEndLocation` (`.Location` (`GameplayStatics.BreakHitResult` _outhit))))
              (bind _movecomp (`ProjBase.MoveComp` _returnvalue))
              (set `MovementComponent.Velocity` (* (`KismetMathLibrary.Normal` (- _output_get_4 (`self.ProjStartLocation`))) (`self.ProjVelocityNum`)) _movecomp)
              (else
                (bind _output_get_5 (set `self.ProjEndLocation` (`KismetMathLibrary.Conv_RotatorToVector` (`SceneComponent.K2_GetComponentRotation` (`self.FollowCamera`)))))
                (set `MovementComponent.Velocity` (* (`KismetMathLibrary.Normal` _output_get_5) (`self.ProjVelocityNum`)) _movecomp)))
            (`KismetSystemLibrary.K2_SetTimerDelegate` (delegate `DestorySelf`) 5.0)))
        (elif (`self.InState2`)
          (`|PlayMontage` (`self.Mesh`) "/Game/OldSheepWorld/Blueprints/Montage/PlayerCharacter/AM_Rifle_Fire_Montage.AM_Rifle_Fire_Montage" 1.0 0.0 "start"
            (:`OnCompleted`
              (set `self.IsPrimaryAttackCooldown` false))
            (:`OnNotifyBegin`
              (bind _returnvalue_3 (`|SpawnActorFromClass` "/Game/OldSheepWorld/Blueprints/BP_PrimaryProj.BP_PrimaryProj_C" (`KismetMathLibrary.Conv_VectorToTransform` (`SceneComponent.K2_GetComponentLocation` (`self.ProjSpawnPosition`))) "Undefined" "OverrideRootScale" null null))
              (set `self.ProjStartLocation` (`SceneComponent.K2_GetComponentLocation` (`self.FollowCamera`)))
              (bind _output_get_6 (set `self.ProjEndLocation` (`KismetMathLibrary.Conv_RotatorToVector` (`SceneComponent.K2_GetComponentRotation` (`self.FollowCamera`)))))
              (bind _output_get_7 (set `self.LineTraceDistance` 10000))
              (bind _output_get_8 (set `self.ProjEndLocation` (+ (* _output_get_7 (`KismetMathLibrary.Normal` _output_get_6)) (`self.ProjStartLocation`))))
              (bind (_outhit_2 _returnvalue_4) (`KismetSystemLibrary.LineTraceSingle` (`self.ProjStartLocation`) _output_get_8 "TraceTypeQuery2"))
              (set `self.ProjStartLocation` (`SceneComponent.K2_GetComponentLocation` (`self.ProjSpawnPosition`)))
              (if _returnvalue_4
                (bind _output_get_9 (set `self.ProjEndLocation` (`.Location` (`GameplayStatics.BreakHitResult` _outhit_2))))
                (bind _movecomp_2 (`ProjBase.MoveComp` _returnvalue_3))
                (set `MovementComponent.Velocity` (* (`KismetMathLibrary.Normal` (- _output_get_9 (`self.ProjStartLocation`))) (`self.ProjVelocityNum`)) _movecomp_2)
                (else
                  (bind _output_get_10 (set `self.ProjEndLocation` (`KismetMathLibrary.Conv_RotatorToVector` (`SceneComponent.K2_GetComponentRotation` (`self.FollowCamera`)))))
                  (set `MovementComponent.Velocity` (* (`KismetMathLibrary.Normal` _output_get_10) (`self.ProjVelocityNum`)) _movecomp_2)))
              (`KismetSystemLibrary.K2_SetTimerDelegate` (delegate `DestorySelf`) 5.0)))
          (elif (`self.InState3`)
            _))))))

(event `DestorySelf`
  (`/Engine/EditorBlueprintResources/StandardMacros.IsValid` (stale `EnhancedInput|/Game/OldSheepWorld/Input/Actions/IA_PrimaryAttack` _returnvalue_3)
    (:`Is Valid`
      (`ProjBase.Explode` (stale `EnhancedInput|/Game/OldSheepWorld/Input/Actions/IA_PrimaryAttack` _returnvalue_3))
      (`KismetSystemLibrary.PrintString` "Explode"))))

(fn `GetHealth`
  (returns (Health :type "Float (double-precision)"))
  (return (`self.Health`)))

(fn `GetMaxHealth`
  (returns (Health :type "Float (double-precision)"))
  (return (`self.MaxHealth`)))

(fn `UserConstructionScript`)