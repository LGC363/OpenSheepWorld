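; Game mode for OldSheepWorld that spawns Countess characters as enemies in waves at the level's TargetPoints.
; On BeginPlay it caches every TargetPoint and starts a looping timer that spawns one enemy at each point's location.
; MaxEnemyNum counts down with each spawn and is never replenished here, so it caps total spawns while the timer keeps firing.
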(event `self.ReceiveBeginPlay`
  (bind _outactors (`GameplayStatics.GetAllActorsOfClass` "/Script/Engine.TargetPoint"))
  (set `self.SpawnPoses` _outactors)
  (`KismetSystemLibrary.K2_SetTimerDelegate` (delegate `SpawnEnemy`) 10.0 true))

(event `SpawnEnemy`
  (for _array_element (`self.SpawnPoses`)
    (if (not (<= (`self.MaxEnemyNum`) 0))
      (`|SpawnActorFromClass` "/Game/OldSheepWorld/Blueprints/AI/Countess/CountessPlayerCharacter.CountessPlayerCharacter_C" (`KismetMathLibrary.Conv_VectorToTransform` (`self.K2_GetActorLocation` _array_element)) "Undefined" "OverrideRootScale" null null)
      (set `self.MaxEnemyNum` (- (`self.MaxEnemyNum`) 1)))))

(fn `UserConstructionScript`)