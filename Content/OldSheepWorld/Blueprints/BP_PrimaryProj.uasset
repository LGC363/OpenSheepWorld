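; BP_PrimaryProj is a projectile, apparently for the player's primary attack, that damages enemies and explodes on a timer.
; On BeginPlay it starts a five-second timer that calls Explode and prints a debug string.
; Sphere collision hits apply fixed damage to actors tagged Enemy, crediting the player character as causer, without triggering the explosion.
; Explode is called but not defined in these graphs.
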(event `self.ReceiveBeginPlay`
  (`KismetSystemLibrary.K2_SetTimerDelegate` (delegate `DestorySelf`) 5.0))

(event `DestorySelf`
  (`/Engine/EditorBlueprintResources/StandardMacros.IsValid` self
    (:`Is Valid`
      (`self.Explode`)
      (`KismetSystemLibrary.PrintString` "Explode"))))

(event `self.SphereComp.OnComponentHit`
  (params (HitComponent :type "PrimitiveComponent Object Reference") (OtherActor :type "Actor Object Reference") (OtherComp :type "PrimitiveComponent Object Reference") (NormalImpulse :type "Vector Structure") (Hit :type "HitResult Structure (by ref)"))
  (if (`self.ActorHasTag` OtherActor "Enemy")
    (`GameplayStatics.ApplyDamage` OtherActor 20.0 null (`GameplayStatics.GetPlayerCharacter` 0))))

(fn `UserConstructionScript`)